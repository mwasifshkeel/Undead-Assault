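; BP_Zombie is a 2D side-scroller Paper2D enemy that hurts the player on contact and awards score when killed.
; Capsule overlaps with the player or gun set a flag, which Tick uses to switch idle/attack flipbooks and apply Delay-throttled damage.
; DamageTakingSystem lowers health, but its death check subtracts damage again.
; Death unpossesses the zombie without destroying it, as does touching a TriggerBox.
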(event OnComponentEndOverlap(CapsuleComponent)
  (params (OverlappedComponent :type Primitive%20Component%20Object%20Reference) (OtherActor :type Actor%20Object%20Reference) (OtherComp :type Primitive%20Component%20Object%20Reference) (OtherBodyIndex :type Integer))
  (Utilities|Casting|CastTo2DSideScrollerCharacter OtherActor
    (:then
      (Variables|Default|SetIsOverlappingPlayer false))
    (:CastFailed
      (Utilities|Casting|CastToUGun OtherActor)
      (Variables|Default|SetIsOverlappingPlayer false))))

(event OnComponentBeginOverlap(CapsuleComponent)
  (params (OverlappedComponent :type Primitive%20Component%20Object%20Reference) (OtherActor :type Actor%20Object%20Reference) (OtherComp :type Primitive%20Component%20Object%20Reference) (OtherBodyIndex :type Integer) (bFromSweep :type Boolean) (SweepResult :type Hit%20Result%20Structure%20%28by%20ref%29))
  (Utilities|Casting|CastTo2DSideScrollerCharacter OtherActor
    (:then
      (Variables|Default|SetIsOverlappingPlayer true))
    (:CastFailed
      (Utilities|Casting|CastToUGun OtherActor
        (:then
          (Variables|Default|SetIsOverlappingPlayer true))
        (:CastFailed
          (Utilities|Casting|CastToTriggerBox OtherActor)
          (Pawn|UnPossess (Pawn|GetController)))))))

(event Custom|Damage%20Taking%20System
  (params (DmgOut :type Integer))
  (Variables|Default|SetHealth (- (Variables|Default|GetHealth) DmgOut))
  (if (<= (- (Variables|Default|GetHealth) DmgOut) 0)
    (bind _as2dside_scroller_character (Utilities|Casting|CastTo2DSideScrollerCharacter (Game|GetPlayerCharacter 0)))
    (Class|TwoDSideScrollerCharacter|SetScore _as2dside_scroller_character (+ (Class|TwoDSideScrollerCharacter|GetScore _as2dside_scroller_character) 100))
    (Pawn|UnPossess (Pawn|GetController))))

(event Custom|UpdateAnimation
  (switch Utilities|FlowControl|Switch|SwitchonEnum_CharacterAnimation (Variables|Default|GetZombieEnum)
    (:NewEnumerator0
      (Sprite|SetFlipbook (Variables|Default|GetPaperFlipbook) "/Game/Sprites/Enemies/Zombie/Zombie_Movement.Zombie_Movement"))
    (:NewEnumerator2
      (Sprite|SetFlipbook (Variables|Default|GetPaperFlipbook) "/Game/Sprites/Enemies/Zombie/Sprites/Shooting/FB_ZombieHitting.FB_ZombieHitting"))))

(event EventBeginPlay)

(event EventTick
  (params (DeltaSeconds :type Float%20%28single-precision%29))
  (Utilities|FlowControl|Sequence
    (:then_0
      (CallFunction|UpdateAnimation))
    (:then_1
      _))
  (if (Variables|Default|GetIsOverlappingPlayer)
    (Variables|Default|SetZombieEnum "NewEnumerator2")
    (bind _as2dside_scroller_character (Utilities|Casting|CastTo2DSideScrollerCharacter (Game|GetPlayerCharacter 0)))
    (Utilities|FlowControl|Delay 0.75)
    (Default|DamageSystem _as2dside_scroller_character 10)
    (else
      (Utilities|FlowControl|Delay 2.2)
      (Variables|Default|SetZombieEnum "NewEnumerator0"))))

(fn ConstructionScript)