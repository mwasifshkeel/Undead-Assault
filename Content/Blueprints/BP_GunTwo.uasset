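; BP_GunTwo is a pickup gun for the 2D side-scroller character, with its own magazine and reserve ammo.
; Shoot is fire-rate gated by a Tick timer, spawns BP_BulletTwo at the Arrow and plays sound at the sound manager's volume.
; An empty magazine or ReloadSystem triggers a delayed refill from reserve.
; Box overlap adds it to inventory, attaching it to the hand if first, otherwise parking it far away.
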(event OnComponentBeginOverlap(Box)
  (params (OverlappedComponent :type Primitive%20Component%20Object%20Reference) (OtherActor :type Actor%20Object%20Reference) (OtherComp :type Primitive%20Component%20Object%20Reference) (OtherBodyIndex :type Integer) (bFromSweep :type Boolean) (SweepResult :type Hit%20Result%20Structure%20%28by%20ref%29))
  (bind _self self)
  ;[1 1 1] Add Gun to Inventory
  (if (Utilities|IsValid OtherActor)
    (bind _as2dside_scroller_character (Utilities|Casting|CastTo2DSideScrollerCharacter OtherActor))
    (if (Class|DoublyLinkedList|IsEmpty (Variables|/Game/2DSideScrollerBP/Blueprints/2DSideScrollerCharacter.2DSideScrollerCharacter_C|GetGunInventory _as2dside_scroller_character))
      (Default|AddGuntoInventory _as2dside_scroller_character _self)
      (Transformation|SetActorLocation (Transformation|GetWorldLocation (Variables|/Script/DSAFinalProject.TwoDSideScrollerCharacter|GetHandComponent _as2dside_scroller_character)) false false)
      (Transformation|AttachComponentToComponent (Variables|/Script/DSAFinalProject.TwoDSideScrollerCharacter|GetHandComponent _as2dside_scroller_character) "None" "SnapToTarget" "SnapToTarget" "SnapToTarget" true)
      (else
        (Transformation|SetActorLocation "5000.000000,5000.000000,5000.000000" false false)
        (Default|AddGuntoInventory _as2dside_scroller_character _self)))))

(event Custom|Shoot
  (bind _returnvalue (Class|UGun|GetGunAmmo))
  (bind _returnvalue_2 (Class|UGun|GetMaxAmmo))
  ;[1 1 1] Shooting
  (if (> (Class|UGun|GetGunAmmo) 0)
    (if (>= (Variables|Default|GetTimeSinceLastShot) (Variables|Default|GetFire%20Rate))
      (Utilities|FlowControl|Sequence
        (:then_0
          (bind _asbp_sound_manager (Utilities|Casting|CastToBP_SoundManager (Game|GetGameInstance)))
          (Audio|PlaySoundatLocation "/Game/Audio/Explosion01.Explosion01" "0, 0, 0" "0, 0, 0" (Variables|/Game/Blueprints/BP_SoundManager.BP_SoundManager_C|GetGunVolume _asbp_sound_manager) 1.0 0.0 0 0 0))
        (:then_1
          (Game|SpawnActorfromClass "/Game/Blueprints/BP_BulletTwo.BP_BulletTwo_C" (Transformation|GetWorldTransform (Variables|Default|GetArrow)) "Undefined" 0 0))
        (:then_2
          (Variables|Default|SetTimeSinceLastShot 0.0))
        (:then_3
          (Class|UGun|SetGunAmmo (- (Class|UGun|GetGunAmmo) 1)))))
    (else
      ;[1 1 1] Reload System
      (if (< _returnvalue 25)
        (Utilities|FlowControl|Delay 1.0)
        (bind _output_get (Variables|Default|SetTransferAmmo (Math|Integer|Min(Integer) (- 25 _returnvalue) _returnvalue_2)))
        (Utilities|FlowControl|Sequence
          (:then_0
            (Class|UGun|SetGunAmmo (+ _returnvalue _output_get)))
          (:then_1
            (Class|UGun|SetMaxAmmo (- _returnvalue_2 _output_get))))))))

(event Custom|Reload%20System
  (bind _returnvalue (Class|UGun|GetGunAmmo))
  (bind _returnvalue_2 (Class|UGun|GetMaxAmmo))
  ;[1 1 1] Reload System
  (if (> (Class|UGun|GetMaxAmmo) 0)
    (if (< _returnvalue 25)
      (Utilities|FlowControl|Delay 1.0)
      (bind _output_get (Variables|Default|SetTransferAmmo (Math|Integer|Min(Integer) (- 25 _returnvalue) _returnvalue_2)))
      (Utilities|FlowControl|Sequence
        (:then_0
          (Class|UGun|SetGunAmmo (+ _returnvalue _output_get)))
        (:then_1
          (Class|UGun|SetMaxAmmo (- _returnvalue_2 _output_get)))))))

(event EventBeginPlay
  (Class|UGun|SetMaxAmmo 200)
  (Class|UGun|SetGunAmmo 25))

(event Collision|EventActorBeginOverlap
  (params (OtherActor :type Actor%20Object%20Reference)))

(event EventTick
  (params (DeltaSeconds :type Float%20%28single-precision%29))
  (Variables|Default|SetTimeSinceLastShot (+ (Variables|Default|GetTimeSinceLastShot) DeltaSeconds)))

(fn ConstructionScript)