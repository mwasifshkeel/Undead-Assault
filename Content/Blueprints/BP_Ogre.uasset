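; BP_Ogre is a 2D side-scroller enemy that damages the player in close range and awards score when defeated.
; Capsule overlaps with the player or gun set a flag; Tick uses it to switch a two-state enum driving flipbooks, with Delays pacing damage and return to idle.
; Damage lowers health, then subtracts again in the death check; death, or leaving a TriggerBox, unpossesses the controller without destroying the actor.
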(event OnComponentBeginOverlap(CapsuleComponent)
  (params (OverlappedComponent :type Primitive%20Component%20Object%20Reference) (OtherActor :type Actor%20Object%20Reference) (OtherComp :type Primitive%20Component%20Object%20Reference) (OtherBodyIndex :type Integer) (bFromSweep :type Boolean) (SweepResult :type Hit%20Result%20Structure%20%28by%20ref%29))
  (Utilities|Casting|CastTo2DSideScrollerCharacter OtherActor
    (:then
      (Variables|Default|SetIsOverlappingPlayer true))
    (:CastFailed
      (Utilities|Casting|CastToUGun OtherActor)
      (Variables|Default|SetIsOverlappingPlayer true))))

(event OnComponentEndOverlap(CapsuleComponent)
  (params (OverlappedComponent :type Primitive%20Component%20Object%20Reference) (OtherActor :type Actor%20Object%20Reference) (OtherComp :type Primitive%20Component%20Object%20Reference) (OtherBodyIndex :type Integer))
  (Utilities|Casting|CastTo2DSideScrollerCharacter OtherActor
    (:then
      (Variables|Default|SetIsOverlappingPlayer false))
    (:CastFailed
      (Utilities|Casting|CastToUGun OtherActor
        (:then
          (Variables|Default|SetIsOverlappingPlayer false))
        (:CastFailed
          (Utilities|Casting|CastToTriggerBox OtherActor)
          (Pawn|UnPossess (Pawn|GetController)))))))

(event Custom|Damage%20Taking%20System
  (params (DmgOut :type Integer))
  ;[1 1 1] Comment
  (Variables|Default|SetHealth (- (Variables|Default|GetHealth) DmgOut))
  (if (<= (- (Variables|Default|GetHealth) DmgOut) 0)
    (bind _as2dside_scroller_character (Utilities|Casting|CastTo2DSideScrollerCharacter (Game|GetPlayerCharacter 0)))
    (Class|TwoDSideScrollerCharacter|SetScore _as2dside_scroller_character (+ (Class|TwoDSideScrollerCharacter|GetScore _as2dside_scroller_character) 1000))
    (Pawn|UnPossess (Pawn|GetController))))

(event Custom|UpdateAnimation
  ;[1 1 1] FSM For Character
  (switch Utilities|FlowControl|Switch|SwitchonEnum_CharacterAnimation (Variables|Default|GetOgreEnum)
    (:NewEnumerator0
      (Sprite|SetFlipbook (Variables|Default|GetPaperFlipbook) "/Game/Sprites/Enemies/Ogre/FB_OgreWalk.FB_OgreWalk"))
    (:NewEnumerator2
      (Sprite|SetFlipbook (Variables|Default|GetPaperFlipbook) "/Game/Sprites/Enemies/Ogre/FB_OgreAttack.FB_OgreAttack"))))

(event Collision|EventActorBeginOverlap
  (params (OtherActor :type Actor%20Object%20Reference)))

(event EventTick
  (params (DeltaSeconds :type Float%20%28single-precision%29))
  ;[1 1 1] Tick - Updates animation
  (Utilities|FlowControl|Sequence
    (:then_0
      (CallFunction|UpdateAnimation))
    (:then_1
      (if (Variables|Default|GetIsOverlappingPlayer)
        (Variables|Default|SetOgreEnum "NewEnumerator2")
        (bind _as2dside_scroller_character (Utilities|Casting|CastTo2DSideScrollerCharacter (Game|GetPlayerCharacter 0)))
        (Utilities|FlowControl|Delay 0.75)
        (Default|DamageSystem _as2dside_scroller_character 20)
        (else
          (Utilities|FlowControl|Delay 2.2)
          (Variables|Default|SetOgreEnum "NewEnumerator0"))))))

(fn ConstructionScript)