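; BP_BulletThree is a bullet actor that damages zombies and ogres and notifies crates it hits.
; Its sphere overlap casts the other actor to each type, applying fixed damage through DamageTakingSystem or calling BulletHit on crates.
; Zombie and ogre hits destroy the bullet, while crate hits do not.
; Tick accumulates a TTL timer that destroys the bullet after a short lifetime.
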(event OnComponentBeginOverlap(Sphere)
  (params (OverlappedComponent :type Primitive%20Component%20Object%20Reference) (OtherActor :type Actor%20Object%20Reference) (OtherComp :type Primitive%20Component%20Object%20Reference) (OtherBodyIndex :type Integer) (bFromSweep :type Boolean) (SweepResult :type Hit%20Result%20Structure%20%28by%20ref%29))
  (Utilities|FlowControl|Sequence
    (:then_0
      (bind _asbp_zombie (Utilities|Casting|CastToBp_Zombie OtherActor))
      (Default|DamageTakingSystem _asbp_zombie 75)
      (Actor|DestroyActor))
    (:then_1
      (bind _asbp_crate (Utilities|Casting|CastToBP_Crate OtherActor))
      (Default|BulletHit _asbp_crate))
    (:then_2
      (bind _asbp_ogre (Utilities|Casting|CastToBP_Ogre OtherActor))
      (Default|DamageTakingSystem _asbp_ogre 75)
      (Actor|DestroyActor))))

(event EventBeginPlay)

(event Collision|EventActorBeginOverlap
  (params (OtherActor :type Actor%20Object%20Reference)))

(event EventTick
  (params (DeltaSeconds :type Float%20%28single-precision%29))
  (Utilities|FlowControl|Sequence
    (:then_0
      (Variables|Default|SetTTL (+ (Variables|Default|GetTTL) DeltaSeconds)))
    (:then_1
      (if (> (Variables|Default|GetTTL) 2.0)
        (Actor|DestroyActor)))))

(fn ConstructionScript)