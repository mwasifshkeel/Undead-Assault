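; AI controller for Bp_Zombie pawns that makes the zombie chase the first player along the X axis.
; While possessing, Tick checks that the player is within horizontal X and vertical Z range, then lerps the pawn's location directly without sweep and turns its yaw toward the player.
; Offsetposition keeps the target slightly short of the player on the zombie's side.
; Unpossessing destroys the pawn.
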(event EventUnPossess
  (params (UnpossessedPawn :type Pawn%20Object%20Reference))
  (Variables|Default|SetControlledZomb 0)
  (Actor|DestroyActor UnpossessedPawn)
  (Variables|Default|SetIsPossessing false))

(event EventPossess
  (params (PossessedPawn :type Pawn%20Object%20Reference))
  (bind _asbp_zombie (Utilities|Casting|CastToBp_Zombie PossessedPawn))
  (Variables|Default|SetControlledZomb _asbp_zombie)
  (Variables|Default|SetIsPossessing true))

(event EventTick
  (params (DeltaSeconds :type Float%20%28single-precision%29))
  (bind _returnvalue (Pawn|GetControlledPawn))
  (bind _returnvalue_2 (Game|GetPlayerCharacter 0))
  (bind _returnvalue_3 (Transformation|GetActorLocation _returnvalue))
  (bind _returnvalue_4 (Transformation|GetActorLocation _returnvalue))
  (bind _returnvalue_5 (Transformation|GetActorLocation _returnvalue_2))
  (bind (_x _y _z) (Math|Vector|BreakVector _returnvalue_5))
  (if (Variables|Default|GetIsPossessing)
    (if (and (<= (Math|Float|Absolute(Float) (- (.x _returnvalue_3) _x)) 7e+02) (<= (Math|Float|Absolute(Float) (- (.z _returnvalue_3) _z)) 2e+02))
      (Utilities|FlowControl|Sequence
        (:then_0
          (Transformation|SetActorLocation _returnvalue (Class|EnemyAIController|LerpLocation (Math|Vector|MakeVector (.x _returnvalue_4) (.y _returnvalue_4) (.z _returnvalue_4)) (Math|Vector|MakeVector (CallFunction|Offsetposition _x (.x _returnvalue_4)) (.y _returnvalue_4) (.z _returnvalue_4)) DeltaSeconds 0.6) false false))
        (:then_1
          (Transformation|SetActorRotation _returnvalue (Math|Rotator|MakeRotator 0.0 0.0 (.yaw (Math|Rotator|FindLookatRotation (Math|Vector|MakeVector (.x _returnvalue_4) (.y _returnvalue_4) (.z _returnvalue_4)) _returnvalue_5)))))))))

(fn ConstructionScript)

(fn Offsetposition
  (params (Targetpos :type Float%20%28single-precision%29) (Selfpos :type Float%20%28single-precision%29))
  (if (<= (- Targetpos Selfpos) 0.0)
    (return (- Targetpos -25.0))
    (else
      (return (- Targetpos 25.0)))))