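; AI controller for BP_Ogre that makes the ogre chase the player along the X axis.
; On possess it caches the ogre, and on unpossess it destroys both the pawn and itself.
; While the player is within range on X, Tick lerps the ogre's location without sweep toward an offset short of the player and yaws it to face them.
; Movement sets the transform directly, using no navigation or behavior tree.
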(event EventUnPossess
  (params (UnpossessedPawn :type Pawn%20Object%20Reference))
  (Variables|Default|SetControlledOgre 0)
  (Actor|DestroyActor UnpossessedPawn)
  (Actor|DestroyActor))

(event EventPossess
  (params (PossessedPawn :type Pawn%20Object%20Reference))
  (bind _asbp_ogre (Utilities|Casting|CastToBP_Ogre PossessedPawn))
  (Variables|Default|SetControlledOgre _asbp_ogre))

(event EventTick
  (params (DeltaSeconds :type Float%20%28single-precision%29))
  (bind _returnvalue (Pawn|GetControlledPawn))
  (bind _returnvalue_2 (Game|GetPlayerCharacter 0))
  (bind _returnvalue_3 (Transformation|GetActorLocation _returnvalue_2))
  (bind _returnvalue_4 (Transformation|GetActorLocation _returnvalue))
  (bind _x (Math|Vector|BreakVector _returnvalue_3))
  (if (Utilities|IsValid (Variables|Default|GetControlledOgre))
    (if (<= (Math|Float|Absolute(Float) (- (.x (Transformation|GetActorLocation _returnvalue)) _x)) 1e+03)
      (Utilities|FlowControl|Sequence
        (:then_0
          (Transformation|SetActorLocation _returnvalue (Class|EnemyAIController|LerpLocation (Math|Vector|MakeVector (.x _returnvalue_4) (.y _returnvalue_4) (.z _returnvalue_4)) (Math|Vector|MakeVector (CallFunction|Offsetposition _x (.x _returnvalue_4)) (.y _returnvalue_4) (.z _returnvalue_4)) DeltaSeconds 0.5) false false))
        (:then_1
          (Transformation|SetActorRotation _returnvalue (Math|Rotator|MakeRotator 0.0 0.0 (.yaw (Math|Rotator|FindLookatRotation (Math|Vector|MakeVector (.x _returnvalue_4) (.y _returnvalue_4) (.z _returnvalue_4)) _returnvalue_3)))))))))

(fn ConstructionScript)

(fn Offsetposition
  (params (Targetpos :type Float%20%28single-precision%29) (Selfpos :type Float%20%28single-precision%29))
  (if (<= (- Targetpos Selfpos) 0.0)
    (return (- Targetpos -1e+02))
    (else
      (return (- Targetpos 1e+02)))))